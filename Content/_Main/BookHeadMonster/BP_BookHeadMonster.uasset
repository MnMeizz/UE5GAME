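; BookHeadMonster enemy that roams, hunts the player by sight and sound, and performs a jumpscare kill.
; PawnSensing interrupts random AIMoveTo wandering to investigate noises or chase faster, with a retriggerable delay restoring wandering after losing sight.
; Reaching the player locks input and camera onto the monster, while montage notifies drive flashlight break and death screen.
; A separate death event plays a death-camera cutscene ending in the victory screen.
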(event `self.ReceiveTick`
  (params (DeltaSeconds :type "Float (single-precision)"))
  (if (`self.LookCamera`)
    (`Controller.SetControlRotation` (`GameplayStatics.GetPlayerController` 0) (`KismetMathLibrary.RInterpTo` (`self.GetControlRotation` (`self.PlayerRef`)) (`KismetMathLibrary.FindLookAtRotation` (`SceneComponent.K2_GetComponentLocation` (`/Game/_Main/_Player/BP_Player.Camera` (`self.PlayerRef`))) (`SceneComponent.GetSocketLocation` (`self.Mesh`) "lowerarm_l")) (`GameplayStatics.GetWorldDeltaSeconds`) 10.0))))

(event `self.ReceiveBeginPlay`
  ; 开始游戏
  (`|ExecutionSequence`
    (:`then_0`
      (bind _asbp_player (cast `/Game/_Main/_Player/BP_Player` (`GameplayStatics.GetPlayerCharacter` 0)))
      (set `self.PlayerRef` _asbp_player))
    (:`then_1`
      (`self.随机走动`))))

(event `随机走动`
  ; 随机走动
  (`|AIMoveTo` self (`NavigationSystemV1.K2_GetRandomReachablePointInRadius` (`self.K2_GetActorLocation`) 3000.0 null null) null
    (:`OnSuccess`
      _)
    (:`OnFail`
      _))
  (`KismetSystemLibrary.Delay` 3.0)
  (if (not (`self.Searchplayer`))
    (`self.随机走动`)))

(event `怪物死亡`
  (bind _mainui (`/Game/_Main/_Player/BP_Player.MainUi` (`self.PlayerRef`)))
  (`CharacterMovementComponent.DisableMovement` (`self.CharacterMovement`))
  (`ActorComponent.Activate` (`self.ParticleSystem`) false)
  (`PlayerController.SetViewTargetWithBlend` (`GameplayStatics.GetPlayerController` 0) (`ActorComponent.GetOwner` (`self.DeathCamera`)) 0.0 "VTBlend_Linear" 0.0 false)
  (`SceneComponent.SetVisibility` (`self.SpotLight`) true false)
  (`KismetSystemLibrary.Delay` 1.0)
  (`UserWidget.PlayAnimation` _mainui (`/Game/_Main/UI/Wedget/WB_MainUI.黑屏淡出` _mainui) 0.0 1 "Reverse" 0.3 false)
  (`KismetSystemLibrary.Delay` 0.3)
  (`|PlayMontage` (`self.Mesh`) "/Game/_Main/BookHeadMonster/Animations/MutantDying_UE_Montage.MutantDying_UE_Montage"
    (:`then`
      (`KismetSystemLibrary.Delay` 1.9)
      (`GameplayStatics.PlaySound2D` "/Game/_Main/SFX/BookHeadMonster/Hit.Hit" 1.0 1.0 0.0 null null)
      (`KismetSystemLibrary.Delay` 1.0)
      (set `Widget.RenderOpacity` 1.0 (`/Game/_Main/UI/Wedget/WB_MainUI.黑屏` (`/Game/_Main/_Player/BP_Player.MainUi` (`self.PlayerRef`))))
      (`KismetSystemLibrary.Delay` 0.5)
      (`/Game/_Main/UI/Wedget/WB_MainUI.显示胜利界面` (`/Game/_Main/_Player/BP_Player.MainUi` (`self.PlayerRef`))))))

(event `self.PawnSensing.OnSeePawn`
  (params (Pawn :type "Pawn Object Reference"))
  ; 追踪玩家
  (`|ExecutionSequence`
    (:`then_0`
      (set `CharacterMovementComponent.MaxWalkSpeed` 250.0 (`self.CharacterMovement`))
      (`|AIMoveTo` self (0.0 0.0 0.0) Pawn 150.0
        (:`OnSuccess`
          (`/Engine/EditorBlueprintResources/StandardMacros.DoOnce` false
            (:`Completed`
              (`self.跳杀`))))))
    (:`then_1`
      (`KismetSystemLibrary.RetriggerableDelay` 1.0)
      (set `CharacterMovementComponent.MaxWalkSpeed` 125.0 (`self.CharacterMovement`))
      (`self.随机走动`)
      (set `self.Searchplayer` false))))

(event `self.PawnSensing.OnHearNoise`
  (params (Instigator :type "Pawn Object Reference") (Location :type "Vector Structure (by ref)") (Volume :type "Float (single-precision)"))
  ; 声音感应
  (set `self.Searchplayer` true)
  (`|AIMoveTo` self Location null
    (:`OnSuccess`
      (set `self.Searchplayer` false))))

(event `跳杀`
  (bind _playerref (`self.PlayerRef`))
  (bind _mainui (`/Game/_Main/_Player/BP_Player.MainUi` (`self.PlayerRef`)))
  (bind _spotlight (`/Game/_Main/_Player/BP_Player.SpotLight` _playerref))
  (`self.K2_SetActorRotation` (`KismetMathLibrary.FindLookAtRotation` (`self.K2_GetActorLocation`) (`self.K2_GetActorLocation` (`self.PlayerRef`))))
  (`CharacterMovementComponent.DisableMovement` (`self.CharacterMovement`))
  (`self.DisableInput` (`self.PlayerRef`) (`GameplayStatics.GetPlayerController` 0))
  (set `self.LookCamera` true)
  (bind _notifyname (`|PlayMontage` (`self.Mesh`) "/Game/_Main/BookHeadMonster/Animations/MutantSwiping_UE_Montage.MutantSwiping_UE_Montage")
    (:`then`
      (`GameplayStatics.PlaySound2D` "/Game/_Main/SFX/BookHeadMonster/BookHeadMonster.BookHeadMonster" 1.0 1.0 0.0 null null)
      (`CameraComponent.SetFieldOfView` (`/Game/_Main/_Player/BP_Player.Camera` _playerref) 120.0)
      (`SpotLightComponent.SetOuterConeAngle` _spotlight 60.0)
      (if (not (`SceneComponent.IsVisible` _spotlight))
        (`SceneComponent.SetVisibility` _spotlight true false)
        (`GameplayStatics.PlaySound2D` "/Game/_Main/SFX/Flashlight/FlashlightOn.FlashlightOn" 1.0 1.0 0.0 null null)))
    (:`OnNotifyBegin`
      (if (== _notifyname "停止摄像机")
        (set `self.LookCamera` false)
        (elif (== _notifyname "BreakFlashlight")
          (`GameplayStatics.PlaySound2D` "/Game/_Main/SFX/Bulb/BulbBreak.BulbBreak" 1.0 1.0 0.0 null null)
          (`SceneComponent.SetVisibility` (`/Game/_Main/_Player/BP_Player.SpotLight` (`self.PlayerRef`)) false false)
          (`GameplayStatics.PlaySound2D` "/Game/_Main/SFX/BookHeadMonster/Hit.Hit" 1.0 1.0 0.0 null null)
          (`UserWidget.PlayAnimation` _mainui (`/Game/_Main/UI/Wedget/WB_MainUI.黑屏淡出` _mainui) 0.0 1 "Forward" 5.0 false)
          (`KismetSystemLibrary.Delay` 2.0)
          (`/Game/_Main/UI/Wedget/WB_MainUI.显示死亡界面` (`/Game/_Main/_Player/BP_Player.MainUi` (`self.PlayerRef`))))))))

(fn `UserConstructionScript`)