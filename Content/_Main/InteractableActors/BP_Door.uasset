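; BP_Door is an interactable hinged door with optional locking and a configurable mesh, set in the construction script.
; While locked, a still-valid Key reference shows a Chinese "door is locked" message; an invalid one triggers a gated, one-time unlock after a short delay.
; Unlocked interaction toggles the door with sounds and a timeline-driven yaw rotation.
; A dot product against the player's position picks the swing direction.
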(event `/Game/_Main/interface/BPI_interface.OnInteract`
  (params (Player :type "/Game/_Main/_Player/BP_Player Object Reference"))
  (bind _returnvalue (`SceneComponent.K2_GetComponentLocation` (`self.StaticMesh`)))
  (set `self.Player` Player)
  (if (`self.Locked`)
    (`/Engine/EditorBlueprintResources/StandardMacros.IsValid` (`self.Key`)
      (:`Is Valid`
        (`GameplayStatics.PlaySoundAtLocation` "/Game/_Main/SFX/Door/DoorsLocked.DoorsLocked" _returnvalue (struct) 1.0 1.0 0.0 null null null null)
        (`/Game/_Main/UI/Wedget/WB_MainUI.显示文本` (`/Game/_Main/_Player/BP_Player.MainUi` (`self.Player`)) "门已上锁"))
      (:`Is Not Valid`
        (`/Engine/EditorBlueprintResources/StandardMacros.Gate` false :!label _label
          (:`Exit`
            (`GameplayStatics.PlaySoundAtLocation` "/Game/_Main/SFX/Door/Door_Unlocking.Door_Unlocking" _returnvalue (struct) 1.0 1.0 0.0 null null null null)
            (`|ExecutionSequence`
              (:`then_0`
                (`KismetSystemLibrary.Delay` 1.3)
                (set `self.Locked` false))
              (:`then_1`
                (goto _label :!via `Close`)))))))
    (else
      (`self.开门/关门`))))

(event `开门/关门`
  (bind _returnvalue (`SceneComponent.K2_GetComponentLocation` (`self.StaticMesh`)))
  (if (`self.DoorisClosed`)
    (set `self.DoorisClosed` false)
    (`GameplayStatics.PlaySoundAtLocation` "/Game/_Main/SFX/Door/DoorOpen.DoorOpen" _returnvalue (struct) 1.0 1.0 0.0 null null null null)
    (set `self.DotProduct` (`KismetMathLibrary.Dot_VectorVector` (`KismetMathLibrary.Normal` (- (`self.K2_GetActorLocation` self) (`self.K2_GetActorLocation` (`self.Player`)))) (`self.GetActorForwardVector` self)))
    (bind (_direction _alpha) (`Timeline|TL_Door` :!label _label_2)
      (:`Update`
        (`SceneComponent.K2_SetRelativeRotation` (`self.StaticMesh`) (`KismetMathLibrary.RLerp` (struct) (`KismetMathLibrary.MakeRotator` 0.0 0.0 (* (`self.OpenAngle`) (`KismetMathLibrary.SelectFloat` 1.0 -1.0 (>= (`self.DotProduct`) 0.0)))) _alpha) false false)))
    (else
      (set `self.DoorisClosed` true)
      (`GameplayStatics.PlaySoundAtLocation` "/Game/_Main/SFX/Door/DoorClose.DoorClose" _returnvalue (struct) 1.0 1.0 0.0 null null null null)
      (goto _label_2 :!via `Reverse`))))

(fn `UserConstructionScript`
  (`StaticMeshComponent.SetStaticMesh` (`self.StaticMesh`) (`self.DoorMesh`)))