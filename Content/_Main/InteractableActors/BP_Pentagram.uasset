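; Interactable pentagram that plays the ending ritual once the game mode reports no pages left; otherwise it shows a hint and the objective.
; A one-shot sequence uses staggered delays to disable input, throw pages via timeline, brighten the pentagram through a material parameter collection, kill lights, spawn fire, play the screen fade and trigger the BookHead monster's death.
; Tick eases the player's view toward the pentagram's sphere while the camera is locked.
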(event `self.ReceiveTick`
  (params (DeltaSeconds :type "Float (single-precision)"))
  (if (`self.LockCamera`)
    (`Controller.SetControlRotation` (`GameplayStatics.GetPlayerController` 0) (`KismetMathLibrary.RInterpTo` (`Pawn.GetControlRotation` (`self.PlayerRef`)) (`KismetMathLibrary.FindLookAtRotation` (`SceneComponent.K2_GetComponentLocation` (`/Game/_Main/_Player/BP_Player.Camera` (`self.PlayerRef`))) (`SceneComponent.K2_GetComponentLocation` (`self.Sphere`))) (`GameplayStatics.GetWorldDeltaSeconds`) 3.0))))

(event `/Game/_Main/interface/BPI_interface.OnInteract`
  (params (Player :type "/Game/_Main/_Player/BP_Player Object Reference"))
  (bind _page1 (`self.Page1`))
  (bind (_returnvalue_x _returnvalue_y _returnvalue_z) (`KismetMathLibrary.BreakVector` (`SceneComponent.K2_GetComponentLocation` (`self.Sphere`))))
  (bind (_returnvalue_x_2 _returnvalue_y_2 _returnvalue_z_2) (`KismetMathLibrary.BreakVector` (`self.K2_GetActorLocation` (`self.PlayerRef`))))
  (bind _mainui (`/Game/_Main/_Player/BP_Player.MainUi` (`self.PlayerRef`)))
  (bind _mainui_2 (`/Game/_Main/_Player/BP_Player.MainUi` (`self.PlayerRef`)))
  (bind _output_get (set `self.PlayerRef` Player))
  (bind _output_get_2 (set `self.Game Mod Ref` (`/Game/_Main/_Player/BP_Player.GameModRef` _output_get)))
  (if (== (`/Game/_Main/framework/BP_ModeBase.PagesLeft` _output_get_2) 0)
    (`/Engine/EditorBlueprintResources/StandardMacros.DoOnce` false
      (:`Completed`
        (`|ExecutionSequence`
          (:`then_0`
            (`KismetSystemLibrary.Delay` 3.0)
            (bind _outactors (`GameplayStatics.GetAllActorsOfClass` "/Game/_Main/InteractableActors/BP_LightSwtich.BP_LightSwtich_C"))
            (for _array_element _outactors
              (set `/Game/_Main/InteractableActors/BP_LightSwtich.IsWorking?` false _array_element)
              (for _array_element_2 (`/Game/_Main/InteractableActors/BP_LightSwtich.LightsToToggle` _array_element)
                (`SceneComponent.SetVisibility` (`Light.LightComponent` _array_element_2) false false)
                (bind _outactors_2 (`GameplayStatics.GetAllActorsOfClass` "/Game/_Main/InteractableActors/BP_Lamp.BP_Lamp_C"))
                (for _array_element_3 _outactors_2
                  (bind _lampmesh (`/Game/_Main/InteractableActors/BP_Lamp.LampMesh` _array_element_3))
                  (`PrimitiveComponent.SetMaterial` _lampmesh (`/Game/_Main/InteractableActors/BP_Lamp.LightMaterialSlot` _array_element_3) "/Game/_Main/3DModels/HangingLight/Lightoff.Lightoff")
                  (`GameplayStatics.PlaySoundAtLocation` "/Game/_Main/SFX/Bulb/BulbBreak.BulbBreak" (`SceneComponent.K2_GetComponentLocation` _lampmesh) (struct) 1.0 1.0 0.0 null null null null)
                  (`SceneComponent.SetVisibility` (`/Game/_Main/_Player/BP_Player.SpotLight` (`self.PlayerRef`)) false false)))))
          (:`then_1`
            (`KismetSystemLibrary.Delay` 1.5)
            (bind (_direction _alpha) (`Timeline|TL_PentagramBrightness`)
              (:`Update`
                (`KismetMaterialLibrary.SetScalarParameterValue` "/Game/_Main/Effects/MPC_Pentagram.MPC_Pentagram" "Brightness" (`KismetMathLibrary.Lerp` 0.0 1000.0 _alpha)))))
          (:`then_2`
            (`self.DisableInput` (`self.PlayerRef`) (`GameplayStatics.GetPlayerController` 0))
            (set `self.LockCamera` true)
            (`KismetSystemLibrary.Delay` 0.5)
            (`SceneComponent.SetVisibility` (`self.Page1`) true false)
            (`SceneComponent.SetVisibility` (`self.Page3`) true false)
            (`SceneComponent.SetVisibility` (`self.Page2`) true false)
            (`SceneComponent.K2_SetWorldLocation` (`self.Page1`) (`self.K2_GetActorLocation` (`self.PlayerRef`)) false false)
            (bind (_direction_2 _finalalpha _rotationalpha _heightalpha) (`Timeline|TL_ThorwPages`)
              (:`Update`
                (`SceneComponent.K2_SetWorldLocation` _page1 (`KismetMathLibrary.VLerp` (`self.K2_GetActorLocation` (`self.PlayerRef`)) (`KismetMathLibrary.MakeVector` _returnvalue_x _returnvalue_y (`KismetMathLibrary.Lerp` _returnvalue_z_2 (+ _returnvalue_z 0.1) _heightalpha)) _finalalpha) false false)
                (`SceneComponent.K2_SetRelativeRotation` _page1 (`KismetMathLibrary.RLerp` (struct :`Yaw` -80.0) (struct :`Yaw` -30.0) _rotationalpha) false false))))
          (:`then_3`
            (`KismetSystemLibrary.Delay` 3.0)
            (`GameplayStatics.SpawnEmitterAtLocation` "/Game/StarterContent/Particles/P_Fire.P_Fire" (`SceneComponent.K2_GetComponentLocation` (`self.Sphere`)) (struct) (1.0 1.0 1.0) false)
            (`GameplayStatics.PlaySound2D` "/Game/StarterContent/Audio/Fire01_Cue.Fire01_Cue" 1.0 1.0 0.0 null null)
            (`GameplayStatics.PlaySound2D` "/Game/StarterContent/Audio/Fire_Sparks01_Cue.Fire_Sparks01_Cue" 1.0 1.0 0.0 null null))
          (:`then_4`
            (`UserWidget.PlayAnimation` _mainui (`/Game/_Main/UI/Wedget/WB_MainUI.默认光标淡出` _mainui) 0.0 1 "Forward" 1.0 false)
            (`UserWidget.PlayAnimation` _mainui (`/Game/_Main/UI/Wedget/WB_MainUI.交互光标淡出` _mainui) 0.0 1 "Forward" 1.0 false))
          (:`then_5`
            (`KismetSystemLibrary.Delay` 5.0)
            (`GameplayStatics.PlaySound2D` "/Game/_Main/VFX/MonsterDeath.MonsterDeath" 1.0 1.0 0.0 null null)
            (`UserWidget.PlayAnimation` _mainui_2 (`/Game/_Main/UI/Wedget/WB_MainUI.黑屏淡出` _mainui_2) 0.0 1 "Forward" 0.3 false)
            (`KismetSystemLibrary.Delay` 1.5)
            (bind _outactors_3 (`GameplayStatics.GetAllActorsOfClass` "/Game/_Main/BookHeadMonster/BP_BookHeadMonster.BP_BookHeadMonster_C"))
            (`/Game/_Main/BookHeadMonster/BP_BookHeadMonster.怪物死亡` _outactors_3)))))
    (else
      (`|ExecutionSequence`
        (:`then_0`
          (`/Game/_Main/UI/Wedget/WB_MainUI.显示文本` (`/Game/_Main/_Player/BP_Player.MainUi` _output_get) "我需要先找到所有页面..."))
        (:`then_1`
          (`/Game/_Main/_Player/BP_Player.显示目标` (`self.PlayerRef`)))))))

(fn `UserConstructionScript`)