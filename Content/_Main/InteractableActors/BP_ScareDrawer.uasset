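; BP_ScareDrawer is an interactable drawer that springs a one-time spider monster jumpscare when first opened.
; OnInteract alternates open and close with sounds and a timeline sliding the drawer, turning the spider toward the player's camera while opening.
; The first open also plays the spider's animation, then after a short delay plays a scream and lerps it into the camera before destroying it.
; IsJumpscare blocks drawer movement during the scare.
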(event `self.OnInteract`
  (params (Player :type "/Game/_Main/_Player/BP_Player Object Reference"))
  (bind _spidermonsterscreem (`self.SpiderMonsterscreem`))
  (bind _returnvalue (`SceneComponent.K2_GetComponentLocation` (`self.Drawer`)))
  (bind _returnvalue_2 (not (`self.IsJumpscare?`)))
  (bind (_returnvalue_roll _returnvalue_pitch _returnvalue_yaw) (`KismetMathLibrary.BreakRotator` (`KismetMathLibrary.FindLookAtRotation` (`SceneComponent.K2_GetComponentLocation` _spidermonsterscreem) (+ (`SceneComponent.K2_GetComponentLocation` (`/Game/_Main/_Player/BP_Player.Camera` (`self.Player`))) (6.0 0.0 0.0)))))
  (set `self.Player` Player)
  (`/Engine/EditorBlueprintResources/StandardMacros.FlipFlop`
    (:`A`
      (`|ExecutionSequence`
        (:`then_0`
          (`GameplayStatics.PlaySoundAtLocation` "/Game/_Main/SFX/Drawer/DrawerOpen.DrawerOpen" _returnvalue (struct) 1.0 1.0 0.0 null null null null)
          (if _returnvalue_2
            (bind (_direction `_新建轨道_0`) (`Timeline|TL_OpenDrawer` :!label _label)
              (:`Update`
                (`SceneComponent.K2_SetRelativeLocation` (`self.Drawer`) (`KismetMathLibrary.MakeVector` 0.0 (`KismetMathLibrary.Lerp` 0.0 20.0 `_新建轨道_0`)) false false)
                (`/Engine/EditorBlueprintResources/StandardMacros.IsValid` (`self.SpiderMonsterscreem`)
                  (:`Is Valid`
                    (`SceneComponent.K2_SetWorldRotation` _spidermonsterscreem (`KismetMathLibrary.MakeRotator` 0.0 0.0 _returnvalue_yaw) false false)))))))
        (:`then_1`
          (`self.Jumpscare`))))
    (:`B`
      (`GameplayStatics.PlaySoundAtLocation` "/Game/_Main/SFX/Drawer/DrawerClose.DrawerClose" _returnvalue (struct) 1.0 1.0 0.0 null null null null)
      (if _returnvalue_2
        (goto _label :!via `Reverse`)))))

(event `Jumpscare`
  (bind _spidermonsterscreem (`self.SpiderMonsterscreem`))
  (bind _spidermonsterscreem_2 (`self.SpiderMonsterscreem`))
  (bind _returnvalue (`SceneComponent.K2_GetComponentLocation` (`self.SpiderMonsterscreem`)))
  (bind _returnvalue_2 (+ (`SceneComponent.K2_GetComponentLocation` (`/Game/_Main/_Player/BP_Player.Camera` (`self.Player`))) (6.0 0.0 0.0)))
  (bind (_returnvalue_roll _returnvalue_pitch _returnvalue_yaw) (`KismetMathLibrary.BreakRotator` (`KismetMathLibrary.FindLookAtRotation` _returnvalue _returnvalue_2)))
  (`/Engine/EditorBlueprintResources/StandardMacros.DoOnce` false
    (:`Completed`
      (set `self.IsJumpscare?` true)
      (`SkeletalMeshComponent.PlayAnimation` (`self.SpiderMonsterscreem`) "/Game/_Main/3DModels/SpiderMonster/source/SpiderMonsterscreem/SkeletalMeshes/SpiderMonsterscreem_Anim.SpiderMonsterscreem_Anim" false)
      (`KismetSystemLibrary.Delay` 0.3)
      (`GameplayStatics.PlaySound2D` "/Game/_Main/SFX/Jumpscares/SpiderMonsterJumpscare.SpiderMonsterJumpscare" 0.2 1.0 0.0 null null)
      (`|ExecutionSequence`
        (:`then_0`
          (bind (_direction `_新建轨道_0`) (`Timeline|TL_Jumpscare`)
            (:`Update`
              (`/Engine/EditorBlueprintResources/StandardMacros.IsValid` _spidermonsterscreem
                (:`Is Valid`
                  (`SceneComponent.K2_SetWorldLocation` _spidermonsterscreem (`KismetMathLibrary.VLerp` _returnvalue _returnvalue_2 `_新建轨道_0`) false false)
                  (`SceneComponent.K2_SetWorldRotation` _spidermonsterscreem (`KismetMathLibrary.MakeRotator` _returnvalue_roll 0.0 (- _returnvalue_yaw 80.0)) false false))))))
        (:`then_1`
          (`KismetSystemLibrary.Delay` 0.35)
          (set `self.IsJumpscare?` false)
          (`SkeletalMeshComponent.Stop` _spidermonsterscreem_2)
          (`ActorComponent.K2_DestroyComponent` _spidermonsterscreem_2))))))

(fn `UserConstructionScript`)